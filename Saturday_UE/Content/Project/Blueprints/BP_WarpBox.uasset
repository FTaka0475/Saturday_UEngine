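; BP_WarpBox is a two-way teleporter that moves any actor overlapping BoxA or BoxB to the other box.
; Each warp spawns a particle effect at the destination.
; IsWarpfromA and IsWarpfromB stop an immediate bounce back until an end overlap on the receiving box clears them.
; IsWayA and IsWayB can restrict travel to one direction by blocking entry from the opposite box.
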(event OnComponentBeginOverlap(BoxA)
  (params (OverlappedComponent :type Primitive%20Component%20Object%20Reference) (OtherActor :type Actor%20Object%20Reference) (OtherComp :type Primitive%20Component%20Object%20Reference) (OtherBodyIndex :type Integer) (bFromSweep :type Boolean) (SweepResult :type Hit%20Result%20Structure%20%28by%20ref%29))
  (bind _boxb (Variables|Default|GetBoxB))
  (bind _returnvalue (Transformation|GetWorldLocation _boxb))
  (if (not (Variables|Default|GetbIs%20wayB))
    (if (not (Variables|Default|GetbIs%20WarpfromB))
      (Variables|Default|SetbIs%20WarpfromA true)
      (Transformation|SetActorLocation OtherActor _returnvalue false false)
      (Effects|SpawnEmitteratLocation "/Engine/Tutorial/SubEditors/TutorialAssets/TutorialParticleSystem.TutorialParticleSystem" _returnvalue))))

(event OnComponentBeginOverlap(BoxB)
  (params (OverlappedComponent :type Primitive%20Component%20Object%20Reference) (OtherActor :type Actor%20Object%20Reference) (OtherComp :type Primitive%20Component%20Object%20Reference) (OtherBodyIndex :type Integer) (bFromSweep :type Boolean) (SweepResult :type Hit%20Result%20Structure%20%28by%20ref%29))
  (bind _boxa (Variables|Default|GetBoxA))
  (bind _returnvalue (Transformation|GetWorldLocation _boxa))
  (if (not (Variables|Default|GetbIs%20wayA))
    (if (not (Variables|Default|GetbIs%20WarpfromA))
      (Variables|Default|SetbIs%20WarpfromB true)
      (Transformation|SetActorLocation OtherActor _returnvalue false false)
      (Effects|SpawnEmitteratLocation "/Engine/Tutorial/SubEditors/TutorialAssets/TutorialParticleSystem.TutorialParticleSystem" _returnvalue))))

(event OnComponentEndOverlap(BoxA)
  (params (OverlappedComponent :type Primitive%20Component%20Object%20Reference) (OtherActor :type Actor%20Object%20Reference) (OtherComp :type Primitive%20Component%20Object%20Reference) (OtherBodyIndex :type Integer))
  (Variables|Default|SetbIs%20WarpfromB false))

(event OnComponentEndOverlap(BoxB)
  (params (OverlappedComponent :type Primitive%20Component%20Object%20Reference) (OtherActor :type Actor%20Object%20Reference) (OtherComp :type Primitive%20Component%20Object%20Reference) (OtherBodyIndex :type Integer))
  (Variables|Default|SetbIs%20WarpfromA false))

(fn ConstructionScript)