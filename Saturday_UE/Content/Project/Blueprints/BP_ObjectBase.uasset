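; BP_ObjectBase is an actor Blueprint, apparently a base for world objects that react to overlaps and can be destroyed.
; Its Box overlap broadcasts the OverlapBaseEventAction dispatcher with the other actor, which BeginPlay binds to a currently empty handler.
; DestroyObject removes the actor when called.
; Disconnected leftover nodes hold character casts, overlap messages and name-based "PointItem" destruction, none of which run.
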(event OnComponentBeginOverlap(Box)
  (params (OverlappedComponent :type Primitive%20Component%20Object%20Reference) (OtherActor :type Actor%20Object%20Reference) (OtherComp :type Primitive%20Component%20Object%20Reference) (OtherBodyIndex :type Integer) (bFromSweep :type Boolean) (SweepResult :type Hit%20Result%20Structure%20%28by%20ref%29))
  (Default|CallOverlapBaseEventAction OtherActor))

(event Custom|OverlapBaseEventAction_Event
  (params (OverlapActor :type Actor%20Object%20Reference)))

(event EventDestroyObject
  (Actor|DestroyActor))

(event EventBeginPlay
  (EventDispatchers|BindEventtoOverlapBaseEventAction (delegate Custom|OverlapBaseEventAction_Event)))

(fn ConstructionScript)