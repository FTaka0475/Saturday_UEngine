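; BP_Rotate is a spinning group of warp boxes, with one success box and four dead boxes as child actors.
; A timeline started on BeginPlay drives the root component's relative yaw.
; The construction script casts the child actors and passes the WarpSuccess target to the A box and WarpDead to each B box.
; A leftover, unconnected copy of that assignment never runs.
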(event EventBeginPlay
  (|CallParentFunction)
  (bind _z (Timeline|Rotation Play)
    (:Update
      (Transformation|SetRelativeRotation (Variables|Default|GetDefaultSceneRoot) (Math|Rotator|MakeRotator 0.0 0.0 _z) false false))))

(fn ConstructionScript
  (bind _output_get (Variables|Default|SetList (Utilities|Array|MakeArray (Variables|/Script/Engine.ChildActorComponent|GetChildActor (Variables|Default|GetBP_WarpBoxOneB)) (Variables|/Script/Engine.ChildActorComponent|GetChildActor (Variables|Default|GetBP_WarpBoxOneB1)) (Variables|/Script/Engine.ChildActorComponent|GetChildActor (Variables|Default|GetBP_WarpBoxOneB2)) (Variables|/Script/Engine.ChildActorComponent|GetChildActor (Variables|Default|GetBP_WarpBoxOneB3)))))
  (for _array_element _output_get
    (bind _asbp_warp_box_one_b (Utilities|Casting|CastToBP_WarpBoxOneB _array_element))
    (Variables|/Game/Project/Blueprints/BP_WarpBoxOneB.BP_WarpBoxOneB_C|SetWarp _asbp_warp_box_one_b (Variables|Default|GetWarp_Dead))
    (bind _asbp_warp_box_one_a (Utilities|Casting|CastToBP_WarpBoxOneA (Variables|/Script/Engine.ChildActorComponent|GetChildActor (Variables|Default|GetBP_WarpBoxOneA))))
    (Variables|/Game/Project/Blueprints/BP_WarpBoxOneA.BP_WarpBoxOneA_C|SetWarp _asbp_warp_box_one_a (Variables|Default|GetWarp_Success))))